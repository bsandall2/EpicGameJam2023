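; Camera-following infinite ocean actor built from a grid of water plane meshes with distance-based LOD.
; Construction builds the grid and optional far outer plane, using a sequence camera for LOD.
; Tick swaps meshes by player camera distance, wraps tiles around the camera and steps the outer plane along.
; MPC_Ocean receives scale, WPO radius, optional custom time and a cutout position and radius for the materials.
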(event EventBeginPlay)

(event Collision|EventActorBeginOverlap
  (params (OtherActor :type Actor%20Object%20Reference)))

(event EventTick
  (params (DeltaSeconds :type Float%20%28single-precision%29))
  (CallFunction|TimeSet)
  (CallFunction|LOD)
  (CallFunction|InfiniteOcean)
  (CallFunction|MoveOuterPlane)
  (CallFunction|SetOceanAttributes)
  (CallFunction|CutoutFuntion))

(fn ConstructionScript
  (CallFunction|CutoutFuntion)
  (CallFunction|TimeSet)
  (CallFunction|AttributesSetup)
  (CallFunction|GenerateGrid)
  (CallFunction|SetupMaterials)
  (CallFunction|AddOuterPlane)
  (CallFunction|SetOceanAttributes)
  (CallFunction|LODEditor)
  (CallFunction|InfiniteOcean)
  (CallFunction|MoveOuterPlane))

(fn AttributesSetup
  (bind _extent (Variables|GRID|GetExtent))
  (bind _density (Variables|GRID|GetDensity))
  (bind _basescale (Variables|GRID|GetBaseScale))
  (bind _density_2 (Variables|GRID|GetDensity))
  (bind _returnvalue (* _density_2 _extent))
  (bind _returnvalue_2 (/ _basescale _density))
  (bind _returnvalue_3 (* _returnvalue_2 24.0))
  (Utilities|Array|Clear (Variables|Default|GetPlaneArray))
  (Variables|Default|SetAmount _returnvalue)
  (Variables|Default|SetScale _returnvalue_2)
  (Variables|Default|SetSpacing _returnvalue_3)
  (Variables|Default|SetOffset (- (/ (* _returnvalue _returnvalue_3) 2.0) (/ _returnvalue_3 2.0))))

(fn GenerateGrid
  (bind _scale (Variables|Default|GetScale))
  (bind _offset (Variables|Default|GetOffset))
  (for _index (range 0 (- (Variables|Default|GetAmount) 1))
    (Variables|Default|SetLocationX (* _index (Variables|Default|GetSpacing)))
    (for _index_2 (range 0 (- (Variables|Default|GetAmount) 1))
      (Variables|Default|SetLocationY (* _index_2 (Variables|Default|GetSpacing)))
      (Variables|Default|SetFinalLocation (Math|Vector|MakeVector (- (Variables|Default|GetLocationX) _offset) (- (Variables|Default|GetLocationY) _offset) 0.0))
      (bind _returnvalue (AddComponent|AddStaticMeshComponent false (Math|Transform|MakeTransform (Variables|Default|GetFinalLocation) "0, 0, 0" (Math|Vector|MakeVector _scale _scale _scale))))
      (Utilities|Array|Add (Variables|Default|GetPlaneArray) _returnvalue)
      (if (Variables|Materials|GetShadows)
        (Rendering|SetCastShadow _returnvalue true)
        (else
          (Rendering|SetCastShadow _returnvalue false))))))

(fn LOD
  (bind _lodscale (Variables|LOD|GetLODScale))
  (bind _loddistance (Variables|LOD|GetLODDistance))
  (bind _lodbias (Variables|LOD|GetLODBias))
  (bind _returnvalue (* _loddistance _lodbias))
  (for _array_element (Variables|Default|GetPlaneArray)
    (if (> (Math|Vector|Distance(Vector) (Transformation|GetWorldLocation _array_element) (Camera|GetCameraLocation (Game|GetPlayerCameraManager 0))) (* _lodscale (* _returnvalue _lodbias)))
      (Components|StaticMesh|SetStaticMesh _array_element "/Game/CinematicOcean/Meshes/WaterPlane_01.WaterPlane_01")
      (elif (> (Math|Vector|Distance(Vector) (Transformation|GetWorldLocation _array_element) (Camera|GetCameraLocation (Game|GetPlayerCameraManager 0))) (* _lodscale _returnvalue))
        (Components|StaticMesh|SetStaticMesh _array_element "/Game/CinematicOcean/Meshes/WaterPlane_02.WaterPlane_02")
        (elif (> (Math|Vector|Distance(Vector) (Transformation|GetWorldLocation _array_element) (Camera|GetCameraLocation (Game|GetPlayerCameraManager 0))) (* _lodscale _loddistance))
          (Components|StaticMesh|SetStaticMesh _array_element "/Game/CinematicOcean/Meshes/WaterPlane_03.WaterPlane_03")
          (else
            (Components|StaticMesh|SetStaticMesh _array_element "/Game/CinematicOcean/Meshes/WaterPlane_04.WaterPlane_04")))))))

(fn SetupMaterials
  (if (Variables|LOD|GetDebugLODMode)
    (CallFunction|SetPlanesMaterial)
    (else
      (CallFunction|SetPlanesMaterial (Variables|Materials|GetOceanMaterial)))))

(fn SetPlanesMaterial
  (params (Material :type Material%20Interface%20Object%20Reference))
  (for _array_element (Variables|Default|GetPlaneArray)
    (Rendering|Material|SetMaterial _array_element 0 Material)))

(fn InfiniteOcean
  (bind _returnvalue (Game|GetPlayerCameraManager 0))
  (bind _amount (Variables|Default|GetAmount))
  (bind _spacing (Variables|Default|GetSpacing))
  (bind _spacing_2 (Variables|Default|GetSpacing))
  (bind _amount_2 (Variables|Default|GetAmount))
  (bind _returnvalue_2 (Camera|GetCameraLocation _returnvalue))
  (bind _returnvalue_3 (* _amount _spacing))
  (bind _returnvalue_4 (* _amount_2 _spacing_2))
  (bind (_x _y) (Math|Vector|BreakVector _returnvalue_2))
  (for _array_element (Variables|Default|GetPlaneArray)
    (Utilities|FlowControl|Sequence
      (:then_0
        (if (> (Math|Float|Absolute(Float) (- _x (.X (Math|Vector|BreakVector (Transformation|GetWorldLocation _array_element))))) (/ (* (Variables|Default|GetAmount) (Variables|Default|GetSpacing)) 2.0))
          (if (> (.X (Math|Vector|BreakVector (Transformation|GetWorldLocation _array_element))) _x)
            (Transformation|SetWorldLocation _array_element (- (Transformation|GetWorldLocation _array_element) (Math|Vector|MakeVector _returnvalue_4 0.0 0.0)) false false)
            (else
              (Transformation|SetWorldLocation _array_element (+ (Transformation|GetWorldLocation _array_element) (Math|Vector|MakeVector _returnvalue_4 0.0 0.0)) false false)))))
      (:then_1
        (if (> (Math|Float|Absolute(Float) (- (.Y (Math|Vector|BreakVector (Transformation|GetWorldLocation _array_element))) _y)) (/ (* (Variables|Default|GetAmount) (Variables|Default|GetSpacing)) 2.0))
          (if (> (.Y (Math|Vector|BreakVector (Transformation|GetWorldLocation _array_element))) _y)
            (Transformation|SetWorldLocation _array_element (- (Transformation|GetWorldLocation _array_element) (Math|Vector|MakeVector 0.0 _returnvalue_3 0.0)) false false)
            (else
              (Transformation|SetWorldLocation _array_element (+ (Transformation|GetWorldLocation _array_element) (Math|Vector|MakeVector 0.0 _returnvalue_3 0.0)) false false))))))))

(fn AddOuterPlane
  (if (Variables|GRID|GetOuterPlane)
    (bind _returnvalue (AddComponent|AddStaticMeshComponent false (Math|Transform|MakeTransform "0, 0, 0" "0, 0, 0" (Math|Conversions|ToVector(Float) (* (* (Variables|GRID|GetBaseScale) (Variables|GRID|GetExtent)) 0.999)))))
    (bind _output_get (Variables|Default|SetOuterPlaneRef _returnvalue))
    (Rendering|Material|SetMaterial _output_get 0 (Variables|Materials|GetFarOceanMaterial))))

(fn SetOceanAttributes
  (Rendering|Material|SetScalarParameterValue "/Game/CinematicOcean/MaterialParameterCollections/MPC_Ocean.MPC_Ocean" "WPORadius" (* (* (Variables|GRID|GetExtent) (Variables|GRID|GetBaseScale)) 1e+01) :!class /Script/Engine.KismetMaterialLibrary)
  (Rendering|Material|SetScalarParameterValue "/Game/CinematicOcean/MaterialParameterCollections/MPC_Ocean.MPC_Ocean" "GlobalScale" (Variables|Materials|GetGlobalMaterialScale) :!class /Script/Engine.KismetMaterialLibrary))

(fn MoveOuterPlane
  (bind _returnvalue (Game|GetPlayerCameraManager 0))
  (bind _outerplaneref (Variables|Default|GetOuterPlaneRef))
  (bind _spacing (Variables|Default|GetSpacing))
  (bind _spacing_2 (Variables|Default|GetSpacing))
  (bind _outerplaneref_2 (Variables|Default|GetOuterPlaneRef))
  (bind _returnvalue_2 (Camera|GetCameraLocation _returnvalue))
  (bind _returnvalue_3 (Transformation|GetWorldLocation _outerplaneref_2))
  (bind _returnvalue_4 (* _spacing 1.0))
  (bind _returnvalue_5 (* _spacing_2 1.0))
  (bind (_x _y) (Math|Vector|BreakVector _returnvalue_3))
  (bind (_x_2 _y_2) (Math|Vector|BreakVector _returnvalue_2))
  (if (Variables|GRID|GetOuterPlane)
    (Utilities|FlowControl|Sequence
      (:then_0
        (if (> (Math|Float|Absolute(Float) (- _x_2 _x)) (/ (Variables|Default|GetSpacing) 2.0))
          (if (> _x _x_2)
            (Transformation|SetWorldLocation _outerplaneref (- _returnvalue_3 (Math|Vector|MakeVector _returnvalue_5 0.0 0.0)) false false)
            (else
              (Transformation|SetWorldLocation _outerplaneref (+ _returnvalue_3 (Math|Vector|MakeVector _returnvalue_5 0.0 0.0)) false false)))))
      (:then_1
        (if (> (Math|Float|Absolute(Float) (- _y _y_2)) (/ (Variables|Default|GetSpacing) 2.0))
          (if (> _y _y_2)
            (Transformation|SetWorldLocation _outerplaneref (- _returnvalue_3 (Math|Vector|MakeVector 0.0 _returnvalue_4 0.0)) false false)
            (else
              (Transformation|SetWorldLocation _outerplaneref (+ _returnvalue_3 (Math|Vector|MakeVector 0.0 _returnvalue_4 0.0)) false false))))))))

(fn TimeSet
  (if (Variables|Time|GetCustomTime)
    (Rendering|Material|SetScalarParameterValue "/Game/CinematicOcean/MaterialParameterCollections/MPC_Ocean.MPC_Ocean" "UseCustomTime" 1.0 :!class /Script/Engine.KismetMaterialLibrary)
    (Rendering|Material|SetScalarParameterValue "/Game/CinematicOcean/MaterialParameterCollections/MPC_Ocean.MPC_Ocean" "Time" (Variables|Time|GetTime) :!class /Script/Engine.KismetMaterialLibrary)
    (else
      (Rendering|Material|SetScalarParameterValue "/Game/CinematicOcean/MaterialParameterCollections/MPC_Ocean.MPC_Ocean" "UseCustomTime" 0.0 :!class /Script/Engine.KismetMaterialLibrary))))

(fn LODEditor
  (bind _lodscale (Variables|LOD|GetLODScale))
  (bind _loddistance (Variables|LOD|GetLODDistance))
  (bind _lodbias (Variables|LOD|GetLODBias))
  (bind _returnvalue (* _loddistance _lodbias))
  (for _array_element (Variables|Default|GetPlaneArray)
    (if (> (Math|Vector|Distance(Vector) (Transformation|GetWorldLocation _array_element) (Transformation|GetActorLocation (Variables|Sequence|GetSequenceCamera))) (* _lodscale (* _returnvalue _lodbias)))
      (Components|StaticMesh|SetStaticMesh _array_element "/Game/CinematicOcean/Meshes/WaterPlane_01.WaterPlane_01")
      (elif (> (Math|Vector|Distance(Vector) (Transformation|GetWorldLocation _array_element) (Transformation|GetActorLocation (Variables|Sequence|GetSequenceCamera))) (* _lodscale _returnvalue))
        (Components|StaticMesh|SetStaticMesh _array_element "/Game/CinematicOcean/Meshes/WaterPlane_02.WaterPlane_02")
        (elif (> (Math|Vector|Distance(Vector) (Transformation|GetWorldLocation _array_element) (Transformation|GetActorLocation (Variables|Sequence|GetSequenceCamera))) (* _lodscale _loddistance))
          (Components|StaticMesh|SetStaticMesh _array_element "/Game/CinematicOcean/Meshes/WaterPlane_03.WaterPlane_03")
          (else
            (Components|StaticMesh|SetStaticMesh _array_element "/Game/CinematicOcean/Meshes/WaterPlane_04.WaterPlane_04")))))))

(fn CutoutFuntion
  (Rendering|Material|SetVectorParameterValue "/Game/CinematicOcean/MaterialParameterCollections/MPC_Ocean.MPC_Ocean" "CutoutLocation" (Math|Conversions|ToLinearColor(Vector) (Math|Transform|TransformLocation (Transformation|GetActorTransform self) (Variables|Cutout|GetCutoutPosition))) :!class /Script/Engine.KismetMaterialLibrary)
  (Rendering|Material|SetScalarParameterValue "/Game/CinematicOcean/MaterialParameterCollections/MPC_Ocean.MPC_Ocean" "CutoutRadius" (Variables|Cutout|GetCutoutRadius) :!class /Script/Engine.KismetMaterialLibrary))