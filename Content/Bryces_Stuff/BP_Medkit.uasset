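; BP_Medkit is a health pickup that heals the player and destroys itself on touch, but only when health is below max.
; Self-restarting timelines animate the hovering group and spinning symbol.
; An outer detection box toggles a hum and enables Tick-driven yaw turning toward the player.
; It also plays or reverses the case-opening timeline, whose event track flip-flops symbol visibility and the CaseOpen flag.
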(event OnComponentBeginOverlap(PlayerDetectionBox)
  (params (OverlappedComponent :type Primitive%20Component%20Object%20Reference) (OtherActor :type Actor%20Object%20Reference) (OtherComp :type Primitive%20Component%20Object%20Reference) (OtherBodyIndex :type Integer) (bFromSweep :type Boolean) (SweepResult :type Hit%20Result%20Structure%20%28by%20ref%29))
  (Utilities|Casting|CastToBP_Player OtherActor)
  (CallFunction|CaseOpenToggle (Variables|Default|GetCaseOpen))
  (Variables|Default|SetPlayerInRange true)
  (Audio|Components|Audio|SetVolumeMultiplier (Variables|Default|GetMedkit_Hum_SFX_Cue) 1.0 :!class /Script/Engine.AudioComponent))

(event OnComponentEndOverlap(PlayerDetectionBox)
  (params (OverlappedComponent :type Primitive%20Component%20Object%20Reference) (OtherActor :type Actor%20Object%20Reference) (OtherComp :type Primitive%20Component%20Object%20Reference) (OtherBodyIndex :type Integer))
  (Utilities|Casting|CastToBP_Player OtherActor)
  (CallFunction|CaseOpenToggle (Variables|Default|GetCaseOpen))
  (Variables|Default|SetPlayerInRange false)
  (Audio|Components|Audio|SetVolumeMultiplier (Variables|Default|GetMedkit_Hum_SFX_Cue) 0.0 :!class /Script/Engine.AudioComponent))

(event OnComponentBeginOverlap(PlayerPickUpBox)
  (params (OverlappedComponent :type Primitive%20Component%20Object%20Reference) (OtherActor :type Actor%20Object%20Reference) (OtherComp :type Primitive%20Component%20Object%20Reference) (OtherBodyIndex :type Integer) (bFromSweep :type Boolean) (SweepResult :type Hit%20Result%20Structure%20%28by%20ref%29))
  (bind _asbp_player (Utilities|Casting|CastToBP_Player OtherActor))
  (if (< (Variables|/Game/Player/Player_Stats.Player_Stats_C|GetHealth_Current (Variables|/Game/Player/BP_Player.BP_Player_C|GetPlayer_Stats _asbp_player)) (Variables|/Game/Player/Player_Stats.Player_Stats_C|GetHealth_MAX (Variables|/Game/Player/BP_Player.BP_Player_C|GetPlayer_Stats _asbp_player)))
    (Default|Heal (Variables|/Game/Player/BP_Player.BP_Player_C|GetPlayer_Stats _asbp_player) 5e+01)
    (Audio|PlaySound2D "/Game/Audio/SFX/Medkit/Medkit_PickUp_SFX.Medkit_PickUp_SFX" 1.0 1.0 0.0 0 0)
    (Actor|DestroyActor)))

(event Custom|RotatingSymbol
  (bind _spin (Timeline|SymbolSpin PlayFromStart)
    (:Update
      (Transformation|SetRelativeRotation (Variables|Default|GetSymbol) (Math|Rotator|MakeRotator 0.0 0.0 (Math|Float|Lerp (Variables|Default|GetSymbolOrigROT) (Variables|Default|GetSymbolNewROT) _spin)) false false))
    (:Finished
      (CallFunction|RotatingSymbol))))

(event Custom|CaseOpenToggle
  (params (CaseOpen :type Boolean))
  (if (not CaseOpen)
    (bind _open (Timeline|CaseOpenTimeline Play)
      (:Update
        (Transformation|SetRelativeRotation (Variables|Default|GetMedkit_Base_Front) (Math|Rotator|MakeRotator (Math|Float|Lerp (Variables|Default|GetCaseOrigROT) (Variables|Default|GetCaseNewROT) _open) 0.0 0.0) false false))
      (:ToggleSymbol
        (CallFunction|ToggleVisibilySymbol)))
    (else
      (Timeline|CaseOpenTimeline Reverse))))

(event Custom|ToggleVisibilySymbol
  (bind _symbol (Variables|Default|GetSymbol))
  (Utilities|FlowControl|FlipFlop
    (:A
      (Rendering|SetVisibility _symbol true false)
      (Variables|Default|SetCaseOpen true))
    (:B
      (Rendering|SetVisibility _symbol false false)
      (Variables|Default|SetCaseOpen false))))

(event Custom|MedkitLift
  (bind _lift (Timeline|MedkitMovement PlayFromStart)
    (:Update
      (Transformation|SetRelativeLocation (Variables|Default|GetGroup) (Math|Vector|MakeVector 0.0 0.0 (Math|Float|Lerp (Variables|Default|GetGroupOrigPOS) (Variables|Default|GetGroupNewPOS) _lift)) false false))
    (:Finished
      (CallFunction|MedkitLift))))

(event Custom|LookAtPlayer
  (if (Variables|Default|GetPlayerInRange)
    (Transformation|SetRelativeRotation (Variables|Default|GetGroup) (Math|Rotator|MakeRotator 0.0 0.0 (.yaw (Math|Interpolation|RInterpTo (Math|Rotator|MakeRotator 0.0 0.0 (.yaw (Variables|/Script/Engine.SceneComponent|GetRelativeRotation (Variables|Default|GetGroup)))) (Math|Rotator|MakeRotator 0.0 0.0 (+ (.yaw (Math|Rotator|FindLookatRotation (Transformation|GetActorLocation) (Transformation|GetActorLocation (Game|GetPlayerCharacter 0)))) -9e+01)) (Utilities|Time|GetWorldDeltaSeconds) 1.0))) false false)))

(event EventBeginPlay
  (CallFunction|RotatingSymbol)
  (CallFunction|MedkitLift))

(event EventTick
  (params (DeltaSeconds :type Float%20%28single-precision%29))
  (CallFunction|LookatPlayer))

(fn ConstructionScript)