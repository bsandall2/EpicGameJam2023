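; BP_Sword is the player's melee sword, with a timed damage window and a swing trail effect.
; ToggleOverlapOn opens a brief hit window through the CollisionActive flag and collision cube visibility, then closes it automatically.
; While the window is open, CollisionCube begin-overlaps send random damage by TakeDamageMessage to living AI_Enemy_Melee actors only.
; TrailVisible separately shows the trail system and hides it after a short delay.
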(event OnComponentBeginOverlap(CollisionCube)
  (params (OverlappedComponent :type Primitive%20Component%20Object%20Reference) (OtherActor :type Actor%20Object%20Reference) (OtherComp :type Primitive%20Component%20Object%20Reference) (OtherBodyIndex :type Integer) (bFromSweep :type Boolean) (SweepResult :type Hit%20Result%20Structure%20%28by%20ref%29))
  (bind _asai_enemy_melee (Utilities|Casting|CastToAI_Enemy_Melee OtherActor))
  (if (Variables|Default|GetCollisionActive)
    (for _array_element (Utilities|Array|MakeArray OtherActor)
      (if (not (Variables|/Game/Enemies/Base_Classes/Enemy_Health.Enemy_Health_C|GetDead? (Variables|/Game/Enemies/Base_Classes/AI_Enemy_Melee.AI_Enemy_Melee_C|GetEnemy_Health _asai_enemy_melee)))
        (Class|EnemyInterface|TakeDamage(Message) _array_element (Math|Random|RandomFloatinRange 5e+01 (Variables|Default|GetMaxDamageAmount)))))))

(event Custom|TrailVisible
  (Rendering|SetVisibility (Variables|Default|GetNE_Trail_System) true false)
  (Utilities|FlowControl|Delay 0.6)
  (CallFunction|TrailHidden))

(event Custom|TrailHidden
  (Rendering|SetVisibility (Variables|Default|GetNE_Trail_System) false false))

(event Custom|ToggleOverlapOn
  (Rendering|SetVisibility (Variables|Default|GetCollisionCube) true false)
  (Variables|Default|SetCollisionActive true)
  (Utilities|FlowControl|Delay 0.3)
  (CallFunction|ToggleOverlapOFF))

(event Custom|ToggleOverlapOFF
  (Rendering|SetVisibility (Variables|Default|GetCollisionCube) false false)
  (Variables|Default|SetCollisionActive false))

(event EventBeginPlay
  (CallFunction|ToggleOverlapOFF))

(fn ConstructionScript)