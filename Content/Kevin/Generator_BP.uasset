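; Generator objective actor that a player repairs by standing in range while it is active, reporting to GameManager when fixed.
; Start resets the visuals; Sphere overlaps run or pause a looping Counter timer and notify GameManager's event timer.
; Counter advances progress and grows PipeEnergy's Z scale, then hides the ring on completion.
; Sphere1 overlaps toggle the current generator's custom-stencil outline, and Tick turns EventWidget toward the player.
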(event OnComponentBeginOverlap(Sphere)
  (params (OverlappedComponent :type Primitive%20Component%20Object%20Reference) (OtherActor :type Actor%20Object%20Reference) (OtherComp :type Primitive%20Component%20Object%20Reference) (OtherBodyIndex :type Integer) (bFromSweep :type Boolean) (SweepResult :type Hit%20Result%20Structure%20%28by%20ref%29))
  (bind _asbp_player (Utilities|Casting|CastToBP_Player OtherActor))
  (Utilities|IsValid _asbp_player
    (:Is%20Valid
      (if (Variables|Default|GetisActive)
        (Development|PrintString "In Event Range" true true "(R=0.000000,G=1.000000,B=0.053293,A=1.000000)")
        (CallFunction|TimerStarts)
        (bind _asgame_manager (Utilities|Casting|CastToGameManager (Game|GetGameMode)))
        (Default|PauseTimer _asgame_manager)
        (else
          (Development|PrintString "Genrerator Not Working Dickhead Fuck Off" true true "(R=1.000000,G=0.010362,B=0.020309,A=1.000000)"))))))

(event OnComponentEndOverlap(Sphere)
  (params (OverlappedComponent :type Primitive%20Component%20Object%20Reference) (OtherActor :type Actor%20Object%20Reference) (OtherComp :type Primitive%20Component%20Object%20Reference) (OtherBodyIndex :type Integer))
  (bind _asbp_player (Utilities|Casting|CastToBP_Player OtherActor))
  (Utilities|IsValid _asbp_player
    (:Is%20Valid
      (if (Variables|Default|GetisActive)
        (Development|PrintString "Out Event Range" true true "(R=1.000000,G=0.000000,B=0.018721,A=1.000000)")
        (CallFunction|TimerStops)
        (bind _asgame_manager (Utilities|Casting|CastToGameManager (Game|GetGameMode)))
        (Default|GeneratorTimer _asgame_manager)
        (else
          (Development|PrintString "Genrerator Not Working Dickhead Fuck Off" true true "(R=1.000000,G=0.010362,B=0.020309,A=1.000000)"))))))

(event OnComponentBeginOverlap(Sphere1)
  (params (OverlappedComponent :type Primitive%20Component%20Object%20Reference) (OtherActor :type Actor%20Object%20Reference) (OtherComp :type Primitive%20Component%20Object%20Reference) (OtherBodyIndex :type Integer) (bFromSweep :type Boolean) (SweepResult :type Hit%20Result%20Structure%20%28by%20ref%29))
  (if (Variables|Default|GetisActive)
    (Utilities|Casting|CastToBP_Player OtherActor)
    (Variables|Default|SetOutlineOn false)
    (bind _asgame_manager (Utilities|Casting|CastToGameManager (Game|GetGameMode)))
    (Rendering|SetCustomDepthStencilValue (Variables|Generator_BP_C|GetGenerator (Variables|/Game/Blueprints/GameManager.GameManager_C|GetcurrentGenerator _asgame_manager)) 0)))

(event OnComponentEndOverlap(Sphere1)
  (params (OverlappedComponent :type Primitive%20Component%20Object%20Reference) (OtherActor :type Actor%20Object%20Reference) (OtherComp :type Primitive%20Component%20Object%20Reference) (OtherBodyIndex :type Integer))
  (if (Variables|Default|GetisActive)
    (Utilities|Casting|CastToBP_Player OtherActor)
    (Variables|Default|SetOutlineOn true)
    (bind _asgame_manager (Utilities|Casting|CastToGameManager (Game|GetGameMode)))
    (Rendering|SetCustomDepthStencilValue (Variables|Generator_BP_C|GetGenerator (Variables|/Game/Blueprints/GameManager.GameManager_C|GetcurrentGenerator _asgame_manager)) 1)))

(event Custom|Event%20Start
  ;[1 1 1] Do Logic To Start Generator Event and Other Visual Logic
  (Transformation|SetWorldScale3D (Variables|Default|GetPipe_Energy) (Math|Vector|MakeVector 1.0 1.0 0.0))
  (Variables|Default|SetcoreCurrentZ (.z (.scale (Transformation|GetWorldTransform (Variables|Default|GetPipe_Energy)))))
  (Rendering|Material|SetMaterial (Variables|Default|GetGenerator) 0 "/Game/Bryces_Stuff/CustomMeshes/Generator/M_GeneratorOFF.M_GeneratorOFF")
  (Rendering|SetVisibility (Variables|Default|GetRing_TEST) true false)
  (Rendering|SetVisibility (Variables|Default|GeteventWidget) true false))

(event Custom|Counter
  (bind _eventwidget (Variables|Default|GeteventWidget))
  (if (Variables|Default|GetisActive)
    (Rendering|SetVisibility _eventwidget true false)
    (else
      (Rendering|SetVisibility _eventwidget false false)))
  (if (>= (Variables|Default|GetcurrentTimer) (Variables|Default|GetmaxTimer))
    (Variables|Default|SetcurrentTimer (Variables|Default|GetmaxTimer))
    (bind _asgame_manager (Utilities|Casting|CastToGameManager (Game|GetGameMode)))
    (Variables|Default|SetisFixed true)
    (Variables|Default|SetOutlineOn false)
    (Rendering|SetCustomDepthStencilValue (Variables|Default|GetGenerator) 0)
    (Rendering|SetVisibility (Variables|Default|GetRing_TEST) false false)
    (Default|EndGeneratorEvent _asgame_manager)
    (else
      (bind _result (Math|Integer|IncrementInt (Variables|Default|GetcurrentTimer))
        (:%20%20
          (CallFunction|ScaleUp)
          (Development|PrintString (Utilities|String|ToString(Integer) _result)))))))

(event Custom|TimerStops
  (Class|KismetSystemLibrary|PauseTimer 0 "Counter")
  (Development|PrintString "timer paused"))

(event Custom|TimerStarts
  (Utilities|Time|SetTimerbyEvent (delegate Custom|Counter) 0.1 true))

(event Custom|ScaleUp
  (if (not (>= (Variables|Default|GetcoreCurrentZ) 1.0))
    (bind _output_get (Variables|Default|SetcoreCurrentZ (+ (Variables|Default|GetcoreCurrentZ) 0.001667)))
    (Transformation|SetRelativeTransform (Variables|Default|GetPipe_Energy) (Math|Transform|MakeTransform "0, 0, 0" "0, 0, 0" (Math|Vector|MakeVector 1.0 1.0 (.z (.scale (Class|KismetMathLibrary|TInterpto (Math|Transform|MakeTransform "0, 0, 0" "0, 0, 0" (Math|Vector|MakeVector 1.0 1.0 _output_get)) (Math|Transform|MakeTransform "0, 0, 0" "0, 0, 0" (Math|Vector|MakeVector 1.0 1.0 1.0)) 0.0 1.0))))) false false)))

(event EventTick
  (params (DeltaSeconds :type Float%20%28single-precision%29))
  (bind _returnvalue (Game|GetPlayerCharacter 0))
  (bind _eventwidget (Variables|Default|GeteventWidget))
  (bind _returnvalue_2 (Transformation|GetActorLocation _returnvalue))
  (bind _returnvalue_3 (Transformation|GetWorldLocation _eventwidget))
  (bind _returnvalue_4 (Math|Rotator|FindLookatRotation _returnvalue_3 _returnvalue_2))
  (Utilities|IsValid _returnvalue
    (:Is%20Valid
      (Transformation|SetWorldRotation _eventwidget (Math|Rotator|MakeRotator (.roll _returnvalue_4) 0.0 (.yaw _returnvalue_4)) false false))))

(event EventBeginPlay
  (bind _returnvalue (UserInterface|CreateWidget "/Game/UI/GeneratorTimer_Widget.GeneratorTimer_Widget_C"))
  (Variables|Default|Settimerwidget _returnvalue))

(fn ConstructionScript)