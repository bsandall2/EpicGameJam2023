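; Computer_BP is an interactable terminal that sells door openings for player points.
; Overlapping its interaction collider shows a DoorCost widget, created at BeginPlay, and leaving removes it.
; Interact checks player 0's points, writes the reduced total and sets a one-time Opened flag, or prints an insult if short.
; OpenDoor searches all Door_BP actors for a matching pair index, playing an explosion sound at the computer and destroying each match.
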(event OnComponentBeginOverlap(InteractionCollider)
  (params (OverlappedComponent :type Primitive%20Component%20Object%20Reference) (OtherActor :type Actor%20Object%20Reference) (OtherComp :type Primitive%20Component%20Object%20Reference) (OtherBodyIndex :type Integer) (bFromSweep :type Boolean) (SweepResult :type Hit%20Result%20Structure%20%28by%20ref%29))
  (Utilities|Casting|CastToBP_Player OtherActor)
  (Default|PointDisplay (Variables|Default|GetCostWidget) (Variables|Default|GetDoorCost)))

(event OnComponentEndOverlap(InteractionCollider)
  (params (OverlappedComponent :type Primitive%20Component%20Object%20Reference) (OtherActor :type Actor%20Object%20Reference) (OtherComp :type Primitive%20Component%20Object%20Reference) (OtherBodyIndex :type Integer))
  (Utilities|Casting|CastToBP_Player OtherActor)
  (Widget|RemovefromParent (Variables|Default|GetCostWidget)))

(event Custom|OpenDoor
  (bind _outactors (Actor|GetAllActorsOfClass "/Game/Kevin/Door_BP.Door_BP_C"))
  (bind _array_element (Utilities|Array|ForEachLoopwithBreak _outactors)
    (:LoopBody
      (if (== (Variables|/Game/Kevin/Door_BP.Door_BP_C|GetComputerPairIndex _array_element) (Variables|Default|GetDoorPairIndex))
        (Audio|PlaySoundatLocation "/Game/LevelDesign/Audio/Ambience/Explosions__Designed__Futuristic_Explosion_04_SND73980.Explosions__Designed__Futuristic_Explosion_04_SND73980" (Transformation|GetActorLocation) "0, 0, 0" 1.0 1.0 0.0 0 0 0 0)
        (Actor|DestroyActor _array_element)))))

(event EventBeginPlay
  (bind _returnvalue (UserInterface|CreateWidget "/Game/UI/DoorCostWIDGET.DoorCostWIDGET_C"))
  (Variables|Default|SetCostWidget _returnvalue))

(event EventInteract
  (if (not (Variables|Default|Getopened))
    (bind _asbp_player (Utilities|Casting|CastToBP_Player (Game|GetPlayerCharacter 0)))
    (if (>= (Variables|/Game/Player/Player_Stats.Player_Stats_C|GetCurrentPoints (Variables|/Game/Player/BP_Player.BP_Player_C|GetPlayer_Stats _asbp_player)) (Variables|Default|GetDoorCost))
      (Variables|/Game/Player/Player_Stats.Player_Stats_C|SetNewPoints (Variables|/Game/Player/BP_Player.BP_Player_C|GetPlayer_Stats _asbp_player) (- (Variables|/Game/Player/Player_Stats.Player_Stats_C|GetCurrentPoints (Variables|/Game/Player/BP_Player.BP_Player_C|GetPlayer_Stats _asbp_player)) (Variables|Default|GetDoorCost)))
      (Variables|Default|Setopened true)
      (CallFunction|OpenDoor)
      (else
        (Development|PrintString "you broke ass bitch!!!")))))

(fn ConstructionScript)