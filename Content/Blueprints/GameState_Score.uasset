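; GameState_Score is a Blueprint, apparently a game state, that manages the high score save object for the HighScore_SAVE slot.
; On BeginPlay or CheckSave, it loads the slot if present, otherwise creates a save object and calls the same load.
; Nothing writes to the slot, and loading assigns Highscore to itself.
; CheckScore refreshes the save and checks the game mode, but its score logic is empty.
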(event Custom|LoadGame
  (bind _returnvalue (SaveGame|LoadGamefromSlot "HighScore_SAVE"))
  (bind _ashigh_score_save (Utilities|Casting|CastToHighScore_SAVE _returnvalue))
  (Variables|/Game/Blueprints/HighScore_SAVE.HighScore_SAVE_C|SetHighscore _ashigh_score_save (Variables|/Game/Blueprints/HighScore_SAVE.HighScore_SAVE_C|GetHighscore _ashigh_score_save))
  (Variables|Default|SetSaveFile _ashigh_score_save))

(event Custom|CreateSave
  (bind _returnvalue (SaveGame|CreateSaveGameObject "/Game/Blueprints/HighScore_SAVE.HighScore_SAVE_C"))
  (Variables|Default|SetSaveFile _returnvalue)
  (CallFunction|LoadGame))

(event Custom|CheckSave
  (bind _returnvalue (SaveGame|DoesSaveGameExist "HighScore_SAVE"))
  (if _returnvalue
    (CallFunction|LoadGame)
    (else
      (CallFunction|CreateSave))))

(event Custom|CheckScore
  (CallFunction|CheckSave)
  (Utilities|IsValid (Variables|Default|GetSaveFile)
    (:Is%20Valid
      (if (== (Game|GetGameMode) "/Game/Blueprints/GameManager.GameManager")
        _))))

(event EventBeginPlay
  (bind _returnvalue (SaveGame|DoesSaveGameExist "HighScore_SAVE"))
  (if _returnvalue
    (CallFunction|LoadGame)
    (else
      (CallFunction|CreateSave))))

(fn ConstructionScript)